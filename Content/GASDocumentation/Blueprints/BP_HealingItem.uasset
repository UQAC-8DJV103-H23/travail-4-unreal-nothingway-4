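; BP_HealingItem is a single-use pickup that heals a BP_TestHero on overlap through the Gameplay Ability System.
; On authority only, it applies GE_Healing to a living hero's ability system component, then destroys itself.
; A looping timer from BeginPlay also runs this logic via DamageTick, but that event supplies no actor of its own, reading the overlap event's OtherActor.
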(event `self.ReceiveBeginPlay`
  (`KismetSystemLibrary.K2_SetTimerDelegate` (delegate `DamageTick`) 1.0 true))

(event `DamageTick`
  (`/Engine/EditorBlueprintResources/ActorMacros.Switch Has Authority` :!label _label
    (:`Authority`
      (bind _asbp_test_hero (cast `/Game/GASDocumentation/Characters/Hero/BP_TestHero` (stale `self.ReceiveActorBeginOverlap` OtherActor)))
      (bind _returnvalue (`AbilitySystemBlueprintLibrary.GetAbilitySystemComponent` _asbp_test_hero))
      (if (and (`GDCharacterBase.IsAlive` _asbp_test_hero) (`KismetSystemLibrary.IsValid` _returnvalue))
        (`AbilitySystemComponent.BP_ApplyGameplayEffectToSelf` _returnvalue "/Game/GASDocumentation/Characters/Shared/GameplayEffects/GE_Healing.GE_Healing_C" 1.0 (`AbilitySystemComponent.MakeEffectContext` _returnvalue))
        (`self.K2_DestroyActor`)))))

(event `self.ReceiveActorBeginOverlap`
  (params (OtherActor :type "Actor Object Reference"))
  (goto _label))

(fn `UserConstructionScript`)