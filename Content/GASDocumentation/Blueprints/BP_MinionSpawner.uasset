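; BP_MinionSpawner is a server-authoritative wave spawner that places minions at its own transform, starting on BeginPlay.
; Each wave loops until the alive count equals WaveSize, spawning MinionClass entries whose index matches a random roll.
; Each death grants XP to player 0's BP_HeroCharacter and lowers the count.
; When the count empties, WaveSize grows by five and the next wave starts after a delay.
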(event `self.ReceiveBeginPlay`
  (`/Engine/EditorBlueprintResources/ActorMacros.Switch Has Authority`
    (:`Authority`
      (`self.StartNextWave`))))

(event `StartNextWave`
  (while (!= (`self.CurrentMinionAlive`) (`self.WaveSize`))
    (`self.SpawnMinion`)))

(event `SpawnMinion`
  (for (_array_element _array_index) (`self.MinionClass`)
    (if (== _array_index (`KismetMathLibrary.RandomIntegerInRange` 0 (`KismetArrayLibrary.Array_Length` (`self.MinionClass`))))
      (bind _returnvalue (`|SpawnActorFromClass` _array_element (`self.GetTransform`) "AdjustIfPossibleButAlwaysSpawn" "OverrideRootScale" null null))
      (`/Engine/EditorBlueprintResources/StandardMacros.IncrementInt` (`self.CurrentMinionAlive`)
        (:`  `
          (add `GDCharacterBase.OnCharacterDied` _returnvalue (delegate `MinionDied`)))))))

(event `MinionDied`
  (params (Character :type "GDCharacterBase Object Reference"))
  (bind _currentminionalive (`self.CurrentMinionAlive`))
  (bind _asbp_hero_character (cast `/Game/GASDocumentation/Characters/Hero/BP_HeroCharacter` (`GameplayStatics.GetPlayerCharacter` 0)))
  (`/Game/GASDocumentation/Characters/Hero/BP_HeroCharacter.GainXP` _asbp_hero_character (`self.MinionXP`))
  (`/Engine/EditorBlueprintResources/StandardMacros.DecrementInt` _currentminionalive
    (:`  `
      (if (<= _currentminionalive 0)
        (set `self.WaveSize` (+ (`self.WaveSize`) 5))
        (`KismetSystemLibrary.Delay` (`self.RespawnDelay`))
        (`self.StartNextWave`)))))

(fn `UserConstructionScript`)