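; Item spawner actor that keeps one item of a configurable class present at its location, respawning it after it is destroyed.
; On BeginPlay, only the server spawns the item at the spawner's transform, adjusting for collisions but always spawning.
; It binds to the item's OnDestroyed event, waits a configurable respawn delay, then spawns a replacement and repeats the cycle.
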(event `self.ReceiveBeginPlay`
  (`/Engine/EditorBlueprintResources/ActorMacros.Switch Has Authority`
    (:`Authority`
      (`self.ItemSpawn`))))

(event `ItemSpawn`
  (bind _returnvalue (`|SpawnActorFromClass` (`self.ItemClass`) (`self.GetTransform`) "AdjustIfPossibleButAlwaysSpawn" "OverrideRootScale" null null))
  (add `self.OnDestroyed` _returnvalue (delegate `ItemDestroyed`)))

(event `ItemDestroyed`
  (params (DestroyedActor :type "Actor Object Reference"))
  (`KismetSystemLibrary.Delay` (`self.RespawnDelay`))
  (`self.ItemSpawn`))

(fn `UserConstructionScript`)