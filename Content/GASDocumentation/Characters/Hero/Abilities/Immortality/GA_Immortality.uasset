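; GA_Immortality is a hero gameplay ability that applies an immortality gameplay effect to its user.
; On activation it casts the avatar to GDHeroCharacter and commits the ability, cancelling if the commit fails.
; It then applies ImmortalityEffectClass at the ability's level through the hero's ability system component and ends immediately, leaving the behavior to the effect.
; A failed cast stops activation without ending or cancelling the ability.
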(event `self.K2_ActivateAbility`
  (bind _asgdhero_character (cast `GDHeroCharacter` (`self.GetAvatarActorFromActorInfo`)))
  (bind _returnvalue (`self.K2_CommitAbility`))
  (if _returnvalue
    (`AbilitySystemComponent.BP_ApplyGameplayEffectSpecToSelf` (`AbilitySystemBlueprintLibrary.GetAbilitySystemComponent` _asgdhero_character) (`self.MakeOutgoingGameplayEffectSpec` (`self.ImmortalityEffectClass`) (`KismetMathLibrary.Conv_IntToDouble` (`self.GetAbilityLevel`))))
    (`self.K2_EndAbility`)
    (else
      (`self.K2_CancelAbility`))))