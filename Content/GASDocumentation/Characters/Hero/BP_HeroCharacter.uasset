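; Hero character Blueprint that adds XP-based leveling on top of the Gameplay Ability System.
; On BeginPlay and each level-up, it reads the DT_Levels row for the current level and applies max health, stamina and mana bonuses via GE_HeroAttributes SetByCaller tags.
; GainXP checks the threshold; leveling resets XP, applies GE_FullStats and unlocks double jump at level two.
; Level and XP changes are pushed to UI_HUD widgets.
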(event `self.ReceiveBeginPlay`
  (bind _returnvalue (`AbilitySystemBlueprintLibrary.GetAbilitySystemComponent` self))
  (bind _returnvalue_2 (`AbilitySystemComponent.MakeOutgoingSpec` :`self` _returnvalue :`GameplayEffectClass` "/Game/GASDocumentation/Characters/Hero/GE_HeroAttributes.GE_HeroAttributes_C"))
  (bind _returnvalue_3 (`|GetDataTableRow` "/Game/GASDocumentation/Characters/Hero/XP/DT_Levels.DT_Levels" (`KismetStringLibrary.Conv_StringToName` (`KismetStringLibrary.Conv_IntToString` (`self.currentLevel`))))
    (:`then`
      (bind (_level _xptolevelup _bonushealth _bonusstamina _bonusmana) (break `/Game/GASDocumentation/Characters/Hero/XP/FLevels` _returnvalue_3))
      (bind _returnvalue_4 (`AbilitySystemBlueprintLibrary.AssignTagSetByCallerMagnitude` _returnvalue_2 (struct :`TagName` "Data.HeroMaxHealth") (`KismetMathLibrary.Conv_IntToDouble` _bonushealth)))
      (`AbilitySystemComponent.BP_ApplyGameplayEffectSpecToSelf` _returnvalue _returnvalue_4)
      (bind _returnvalue_5 (`AbilitySystemBlueprintLibrary.AssignTagSetByCallerMagnitude` _returnvalue_2 (struct :`TagName` "Data.HeroMaxStamina") (`KismetMathLibrary.Conv_IntToDouble` _bonusstamina)))
      (`AbilitySystemComponent.BP_ApplyGameplayEffectSpecToSelf` _returnvalue _returnvalue_5)
      (bind _returnvalue_6 (`AbilitySystemBlueprintLibrary.AssignTagSetByCallerMagnitude` _returnvalue_2 (struct :`TagName` "Data.HeroMaxMana") (`KismetMathLibrary.Conv_IntToDouble` _bonusmana)))
      (`AbilitySystemComponent.BP_ApplyGameplayEffectSpecToSelf` _returnvalue _returnvalue_6)
      (bind _foundwidgets (`WidgetBlueprintLibrary.GetAllWidgetsOfClass` "/Game/GASDocumentation/UI/UI_HUD.UI_HUD_C"))
      (for _array_element _foundwidgets
        (`/Game/GASDocumentation/UI/UI_HUD.Set Level` _array_element (`self.currentLevel`) _xptolevelup)
        (`KismetSystemLibrary.PrintString` "Hello")))))

(event `GainXP`
  (params (XpToAdd :type Integer))
  (bind _output_get (set `self.currentXP` (+ XpToAdd (`self.currentXP`))))
  (`self.CheckLevelUp`)
  (bind _foundwidgets (`WidgetBlueprintLibrary.GetAllWidgetsOfClass` "/Game/GASDocumentation/UI/UI_HUD.UI_HUD_C"))
  (for _array_element _foundwidgets
    (`/Game/GASDocumentation/UI/UI_HUD.Set XP` _array_element _output_get)))

(event `CheckLevelUp`
  (bind _currentlevel (`self.currentLevel`))
  (bind _returnvalue (`|GetDataTableRow` "/Game/GASDocumentation/Characters/Hero/XP/DT_Levels.DT_Levels" (`KismetStringLibrary.Conv_StringToName` (`KismetStringLibrary.Conv_IntToString` (`self.currentLevel`))))
    (:`then`
      (if (>= (`self.currentXP`) (`.XpToLevelUp_4_C50DE4D3430BF7C4BE44A98F7C5FE9F1` (break `/Game/GASDocumentation/Characters/Hero/XP/FLevels` _returnvalue)))
        (`/Engine/EditorBlueprintResources/StandardMacros.IncrementInt` _currentlevel
          (:`  `
            (set `self.currentXP` 0)
            (`self.LeveledUp`)
            (`self.Unlock Jump` _currentlevel)
            (`KismetSystemLibrary.PrintString` (`KismetStringLibrary.Conv_IntToString` (`self.currentXP`)))))))))

(event `LeveledUp`
  (bind _returnvalue (`AbilitySystemBlueprintLibrary.GetAbilitySystemComponent` self))
  (bind _returnvalue_2 (`AbilitySystemComponent.MakeOutgoingSpec` :`self` _returnvalue :`GameplayEffectClass` "/Game/GASDocumentation/Characters/Hero/GE_HeroAttributes.GE_HeroAttributes_C"))
  (bind _returnvalue_3 (`|GetDataTableRow` "/Game/GASDocumentation/Characters/Hero/XP/DT_Levels.DT_Levels" (`KismetStringLibrary.Conv_StringToName` (`KismetStringLibrary.Conv_IntToString` (`self.currentLevel`))))
    (:`then`
      (bind (_level _xptolevelup _bonushealth _bonusstamina _bonusmana) (break `/Game/GASDocumentation/Characters/Hero/XP/FLevels` _returnvalue_3))
      (bind _returnvalue_4 (`AbilitySystemBlueprintLibrary.AssignTagSetByCallerMagnitude` _returnvalue_2 (struct :`TagName` "Data.HeroMaxHealth") (`KismetMathLibrary.Conv_IntToDouble` _bonushealth)))
      (`AbilitySystemComponent.BP_ApplyGameplayEffectSpecToSelf` _returnvalue _returnvalue_4)
      (bind _returnvalue_5 (`AbilitySystemBlueprintLibrary.AssignTagSetByCallerMagnitude` _returnvalue_2 (struct :`TagName` "Data.HeroMaxStamina") (`KismetMathLibrary.Conv_IntToDouble` _bonusstamina)))
      (`AbilitySystemComponent.BP_ApplyGameplayEffectSpecToSelf` _returnvalue _returnvalue_5)
      (bind _returnvalue_6 (`AbilitySystemBlueprintLibrary.AssignTagSetByCallerMagnitude` _returnvalue_2 (struct :`TagName` "Data.HeroMaxMana") (`KismetMathLibrary.Conv_IntToDouble` _bonusmana)))
      (`AbilitySystemComponent.BP_ApplyGameplayEffectSpecToSelf` _returnvalue _returnvalue_6)
      (`AbilitySystemComponent.BP_ApplyGameplayEffectToSelf` :`self` _returnvalue :`GameplayEffectClass` "/Game/GASDocumentation/Characters/Hero/XP/GE_FullStats.GE_FullStats_C" :`Level` 1.0)
      (bind _foundwidgets (`WidgetBlueprintLibrary.GetAllWidgetsOfClass` "/Game/GASDocumentation/UI/UI_HUD.UI_HUD_C"))
      (for _array_element _foundwidgets
        (`/Game/GASDocumentation/UI/UI_HUD.Set Level` _array_element (`self.currentLevel`) _xptolevelup)
        (`/Game/GASDocumentation/UI/UI_HUD.Set XP` _array_element (`self.currentXP`))
        (`KismetSystemLibrary.PrintString` "Hello")))))

(event `Unlock Jump`
  (params (`Character Level` :type Integer))
  (if (== `Character Level` 2)
    (set `self.JumpMaxCount` 2)))

(fn `UserConstructionScript`)