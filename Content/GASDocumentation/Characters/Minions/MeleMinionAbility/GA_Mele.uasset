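; GA_Mele is a gameplay ability that lets a minion character perform a melee attack.
; On activation it casts the avatar to GDMinionCharacter and commits the ability, cancelling if the commit fails.
; It then spawns a melee zone actor at the minion's mesh, passing it the damage effect class, damage value and instigator, and ends immediately, leaving damage delivery to that actor.
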(event `self.K2_ActivateAbility`
  (bind _owner (`self.Owner`))
  (bind _mesh (`Character.Mesh` _owner))
  (bind _asgdminion_character (cast `GDMinionCharacter` (`self.GetAvatarActorFromActorInfo`)))
  (set `self.Owner` _asgdminion_character)
  (bind _returnvalue (`self.K2_CommitAbility`))
  (if _returnvalue
    (`|SpawnActorFromClass` (`self.MeleZoneClass`) (`KismetMathLibrary.MakeTransform` (`SceneComponent.K2_GetComponentLocation` _mesh) (`SceneComponent.RelativeRotation` _mesh)) "AlwaysSpawn" "OverrideRootScale" _owner (`self.DamageGameplayEffectClass`) (`self.Damage`) _owner)
    (`self.K2_EndAbility`)
    (else
      (`self.K2_CancelAbility`))))

(event `self.K2_OnEndAbility`
  (params (bWasCancelled :type Boolean)))