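; Gameplay Ability for the ranged minion that fires a projectile on activation.
; After committing, it spawns the projectile just ahead of and above the mesh, facing the minion's rotation, passing it the damage effect class and amount.
; It then removes the loose State.Ranged tag from the instigator.
; A failed commit cancels the ability, while the success path never calls EndAbility, whose node is unconnected.
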(event `self.K2_ActivateAbility`
  (bind _owner (`self.Owner`))
  (bind _asgdminion_character (cast `GDMinionCharacter` (`self.GetAvatarActorFromActorInfo`)))
  (set `self.Owner` _asgdminion_character)
  (bind _returnvalue (`self.K2_CommitAbility`))
  (if _returnvalue
    (`|SpawnActorFromClass` (`self.Projectile`) (`KismetMathLibrary.MakeTransform` (+ (`SceneComponent.K2_GetComponentLocation` (`Character.Mesh` _owner)) (+ (* (`Actor.GetActorForwardVector` _owner) (5.0 5.0 5.0)) (* (`Actor.GetActorUpVector` _owner) (0.0 0.0 70.0)))) (`Actor.K2_GetActorRotation` _owner)) "AlwaysSpawn" "OverrideRootScale" _owner (`self.DamageGameplayEffectClass`) (`self.Damage`) 1000.0 (struct) (struct) _owner)
    (`AbilitySystemBlueprintLibrary.RemoveLooseGameplayTags` (`AbilitySystemBlueprintLibrary.GetInstigatorActor` (struct)) (`BlueprintGameplayTagLibrary.MakeGameplayTagContainerFromArray` (`|MakeArray` (struct :`TagName` "State.Ranged") :!type "GameplayTag Structure")))
    (else
      (`self.K2_CancelAbility`))))